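; Save game object that passes itself to saveable objects and keeps typed named variables in a SavedVariables store.
; SaveAllData sends each object a save message and LoadDataForRequester sends a single requester a load message, leaving data handling to the receivers.
; UpdateSaveVariables copies a name-to-value map into the store, switching on int, float, bool, string or string array, and skips names not already present.
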(fn `LoadDataForRequester`
  (params (Requester :type "Object Object Reference"))
  (message `/Game/Save/SaveGame/BPI_Saveable.LoadData` Requester self)
  (return))

(fn `SaveAllData`
  (params (SaveableObjects :type "Array of Object Object Reference"))
  (for _array_element SaveableObjects
    (message `/Game/Save/SaveGame/BPI_Saveable.SaveData` _array_element self))
  (return))

(fn `UpdateSaveVariables`
  (params (Map :type "Map of String to GenericVariable Structure (by ref)"))
  (locals (VariableName :type String))
  (bind (_keypin _valuepin) (`|MapForEach` Map)
    (:`then`
      (bind _returnvalue (`GenericVariableStoreBPLibrary.GV_HasVariable` (`self.SavedVariables`) _keypin))
      (if _returnvalue
        (set `local.VariableName` _keypin)
        (bind (_type _intvalue _floatvalue _boolvalue _stringvalue _stringarrayvalue) (break `GenericVariable` _valuepin))
        (switch `EVariableType` _type
          (:`None`
            _)
          (:`Int`
            (`GenericVariableStoreBPLibrary.GV_SetInt` (`self.SavedVariables`) (`local.VariableName`) _intvalue))
          (:`Float`
            (`GenericVariableStoreBPLibrary.GV_SetFloat` (`self.SavedVariables`) (`local.VariableName`) _floatvalue))
          (:`Bool`
            (`GenericVariableStoreBPLibrary.GV_SetBool` (`self.SavedVariables`) (`local.VariableName`) _boolvalue))
          (:`String`
            (`GenericVariableStoreBPLibrary.GV_SetString` (`self.SavedVariables`) (`local.VariableName`) _stringvalue))
          (:`StringArray`
            (`GenericVariableStoreBPLibrary.GV_SetStringArray` (`self.SavedVariables`) (`local.VariableName`) _stringarrayvalue)))
        (set `local.VariableName` "")))))