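; Checkpoint actor that records itself as the player's last checkpoint when a BP_ElementCharacter enters its overlap area.
; On BeginPlay it replaces its actor tags with its checkpoint name.
; On overlap it writes that name as "LastCheckpoint" to the game instance's global and SaveGame variables, then requests an async save including the current level name.
; GetSpawnLocation exposes the world location of its SpawnPoint component.
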(event `self.ReceiveBeginPlay`
  (`self.SetCheckpointName` (`self.ChekpointName`)))

(event `self.CheckointArea.OnComponentBeginOverlap`
  (params (OverlappedComponent :type "PrimitiveComponent Object Reference") (OtherActor :type "Actor Object Reference") (OtherComp :type "PrimitiveComponent Object Reference") (OtherBodyIndex :type Integer) (bFromSweep :type Boolean) (SweepResult :type "HitResult Structure (by ref)"))
  (cast `/Game/Characters/BP_ElementCharacter` OtherActor)
  (bind _asbp_element_game_instance (cast `/Game/System/BP_ElementGameInstance` (`GameplayStatics.GetGameInstance`)))
  (`GenericVariableStoreBPLibrary.GV_SetString` (`ElementGameInstance.GlobalVariables` _asbp_element_game_instance) "LastCheckpoint" (`KismetStringLibrary.Conv_NameToString` (`self.ChekpointName`)))
  (`GenericVariableStoreBPLibrary.GV_SetString` (`ElementSaveGame.SavedVariables` (`/Game/System/BP_ElementGameInstance.SaveGameRef` _asbp_element_game_instance)) "LastCheckpoint" (`KismetStringLibrary.Conv_NameToString` (`self.ChekpointName`)))
  (`/Game/System/BP_ElementGameInstance.RequestSave` _asbp_element_game_instance true true))

(fn `GetSpawnLocation`
  (returns (ReturnValue :type "Vector Structure"))
  (return (`SceneComponent.K2_GetComponentLocation` (`self.Spawn_Point`))))

(fn `SetCheckpointName`
  (params (ChekpointName :type Name))
  (bind _output_get (set `self.ChekpointName` ChekpointName))
  (set `self.Tags` (`|MakeArray` _output_get)))

(fn `UserConstructionScript`)