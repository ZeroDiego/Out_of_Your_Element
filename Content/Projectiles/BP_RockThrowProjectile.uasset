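; BP_RockThrowProjectile is a thrown rock projectile that stuns and knocks back element characters it hits.
; It binds to the parent's OnProjectileHit event at BeginPlay and applies the GE_HitStun gameplay effect to any ElementCharacterBase hit.
; Unless the target's ability system has the State.Immune.Knockback tag, it launches the target horizontally along the projectile's forward direction, overriding its current velocity.
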(event `self.ReceiveBeginPlay`
  (`parent.ReceiveBeginPlay`)
  (add `ElementProjectileBase.OnProjectileHit` (delegate `OnProjectileHitEvent`)))

(event `OnProjectileHitEvent`
  (params (Projectile :type "ElementProjectileBase Object Reference") (HitActor :type "Actor Object Reference") (ShouldDestory :type "MutableBool Structure"))
  (bind _aselement_character_base (cast `ElementCharacterBase` HitActor))
  (bind _elementabilitysystemcomponent (`ElementCharacterBase.ElementAbilitySystemComponent` _aselement_character_base))
  (`AbilitySystemComponent.BP_ApplyGameplayEffectToSelf` :`self` _elementabilitysystemcomponent :`GameplayEffectClass` "/Game/GameplayEffects/StatusEffects/GE_HitStun.GE_HitStun_C")
  (if (not (`ActorComponent.ComponentHasTag` _elementabilitysystemcomponent "State.Immune.Knockback"))
    (`Character.LaunchCharacter` _aselement_character_base (* (`self.GetActorForwardVector` Projectile) (2000.0 2000.0 0.0)) true true)))

(fn `UserConstructionScript`
  (`parent.UserConstructionScript`))