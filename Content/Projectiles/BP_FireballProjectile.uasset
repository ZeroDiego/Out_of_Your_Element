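; Fireball projectile that sets the element characters it hits on fire with a burning gameplay effect.
; On BeginPlay it binds to its own projectile-hit event and ignores hit actors that are not an ElementCharacterBase.
; It builds a GE_Burning_SetByCaller spec, fills duration and damage through SetByCaller tags with hardcoded values, and applies it to the target's own ability system component.
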(event `self.ReceiveBeginPlay`
  (`parent.ReceiveBeginPlay`)
  (add `ElementProjectileBase.OnProjectileHit` (delegate `OnProjectileHitEvent`)))

(event `OnProjectileHitEvent`
  (params (Projectile :type "ElementProjectileBase Object Reference") (HitActor :type "Actor Object Reference") (ShouldDestory :type "MutableBool Structure"))
  ;[0.1 0 0 0.5] FireDotDamage
  (bind _aselement_character_base (cast `ElementCharacterBase` HitActor))
  (bind _returnvalue (`AbilitySystemBlueprintLibrary.MakeSpecHandleByClass` "/Game/GameplayEffects/StatusEffects/GE_Burning_SetByCaller.GE_Burning_SetByCaller_C"))
  (bind _returnvalue_2 (`AbilitySystemBlueprintLibrary.AssignTagSetByCallerMagnitude` _returnvalue (struct :`TagName` "Abilities.Parameters.Duration") 4.0))
  (bind _returnvalue_3 (`AbilitySystemBlueprintLibrary.AssignTagSetByCallerMagnitude` _returnvalue_2 (struct :`TagName` "Abilities.Parameters.Damage") 5.0))
  (`AbilitySystemComponent.BP_ApplyGameplayEffectSpecToSelf` (`AbilitySystemBlueprintLibrary.GetAbilitySystemComponent` _aselement_character_base) _returnvalue_3))

(fn `UserConstructionScript`
  (`parent.UserConstructionScript`))