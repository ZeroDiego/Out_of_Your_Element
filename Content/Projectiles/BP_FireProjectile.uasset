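; BP_FireProjectile is a fire projectile that applies a damage-over-time effect to the character it hits.
; On BeginPlay it runs the parent logic and binds to the projectile hit delegate.
; On hit it builds a fireball DoT GameplayEffect spec, passing fixed duration and damage through SetByCaller tags.
; It applies the spec to a valid character's AbilitySystemComponent, then destroys itself.
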(event `self.ReceiveBeginPlay`
  (`parent.ReceiveBeginPlay`)
  (add `ElementProjectileBase.OnProjectileHitDelegate` (delegate `OnFireProjectileHit`)))

(event `OnFireProjectileHit`
  (params (HitCharacter :type "ElementCharacterBase Object Reference"))
  ;[0.1 0 0 0.5] FireDotDamage
  (bind _returnvalue (`AbilitySystemBlueprintLibrary.MakeSpecHandleByClass` "/Game/GameplayEffects/Damages/GE_FireballDotDamage_SetByCaller.GE_FireballDotDamage_SetByCaller_C"))
  (bind _returnvalue_2 (`AbilitySystemBlueprintLibrary.AssignTagSetByCallerMagnitude` _returnvalue (struct :`TagName` "Abilities.Parameters.Duration") 4.0))
  (bind _returnvalue_3 (`AbilitySystemBlueprintLibrary.AssignTagSetByCallerMagnitude` _returnvalue_2 (struct :`TagName` "Abilities.Parameters.Damage") 5.0))
  (`/Engine/EditorBlueprintResources/StandardMacros.IsValid` HitCharacter
    (:`Is Valid`
      (`AbilitySystemComponent.BP_ApplyGameplayEffectSpecToSelf` (`AbilitySystemBlueprintLibrary.GetAbilitySystemComponent` HitCharacter) _returnvalue_3))
    (:`Is Not Valid`
      _))
  (`self.K2_DestroyActor`))

(fn `UserConstructionScript`
  (`parent.UserConstructionScript`))