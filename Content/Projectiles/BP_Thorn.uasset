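; Thorn actor that rises at its spawn point with a Niagara effect, deals damage, then retracts.
; BeginPlay gives the skeletal mesh a random yaw and uses ThornDistance as a delay before revealing it and playing a height timeline.
; A delay derived from the remaining lifespan reverses that timeline, while DoDamage, defined outside this graph, fires after ThornDistance plus DamageDelay.
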(event `self.ReceiveBeginPlay`
  (bind _thorndistance (`self.ThornDistance`))
  (set `self.StartLocation` (`self.K2_GetActorLocation`))
  (`|ExecutionSequence`
    (:`then_0`
      (`SceneComponent.K2_SetRelativeRotation` (`self.Thorn Skeletal Mesh`) (`KismetMathLibrary.MakeRotator` 0.0 0.0 (`KismetMathLibrary.RandomFloatInRange` 0.0 360.0)) false false))
    (:`then_1`
      (`KismetSystemLibrary.Delay` _thorndistance)
      (`SceneComponent.SetVisibility` (`self.Thorn Skeletal Mesh`) true false)
      (`ActorComponent.Activate` (`self.NS_Thorn`) false)
      (`|ExecutionSequence`
        (:`then_0`
          (bind (_direction _thorn_height) (`Timeline|Thorn Animation Timeline` :!via `PlayFromStart` :!label _label)
            (:`Update`
              (`SceneComponent.K2_SetRelativeLocation` (`self.Thorn Skeletal Mesh`) (`KismetMathLibrary.MakeVector` 0.0 0.0 _thorn_height) false false))))
        (:`then_1`
          (`KismetSystemLibrary.Delay` (- (`self.GetLifeSpan`) _thorndistance (`TimelineComponent.GetPlaybackPosition` (`self.Thorn Animation Timeline`))))
          (goto _label :!via `Reverse`))))
    (:`then_2`
      (`KismetSystemLibrary.Delay` (+ _thorndistance (`self.DamageDelay`)))
      (`self.DoDamage`))))

(fn `UserConstructionScript`)