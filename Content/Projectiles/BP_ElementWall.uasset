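; BP_ElementWall is an elemental wall actor with its own health attribute set, a nature-wall particle effect and an attached sound.
; On BeginPlay it creates an enemy overlay widget bound to its ElementHealthAttributeSet from the ability system component and places it in the OverlayWidget component.
; It calls DoDamage once after a short delay and destroys itself when the NatureWall particle system finishes.
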(event `self.ReceiveBeginPlay`
  (`GameplayStatics.SpawnSoundAttached` "/Game/Assets/Audio/SoundCues/Abilities/NatureWall_Cue.NatureWall_Cue" (`self.Box`) "None" (0.0 0.0 0.0) (struct) "KeepRelativeOffset" false 1.0 1.0 0.0 null null)
  (bind _returnvalue (`AbilitySystemComponent.GetAttributeSet` (`self.ElementAbilitySystemComponent`) "/Script/Out_of_Your_Element.ElementHealthAttributeSet"))
  (bind _returnvalue_2 (`|CreateWidget` "/Game/UI/World/WBP_EnemyOverlay.WBP_EnemyOverlay_C" null _returnvalue))
  (`WidgetComponent.SetWidget` (`self.OverlayWidget`) _returnvalue_2)
  (add `NiagaraComponent.OnSystemFinished` (`self.NatureWall`) (delegate `OnSystemFinishedEvent`))
  (`KismetSystemLibrary.Delay` 0.5)
  (`self.DoDamage`))

(event `OnSystemFinishedEvent`
  (params (PSystem :type "NiagaraComponent Object Reference"))
  (`self.K2_DestroyActor`))

(fn `UserConstructionScript`)