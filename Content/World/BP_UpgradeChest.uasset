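; Upgrade chest pickup that raises one of the overlapping BP_ElementCharacter's spells to level 2.
; On overlap, FindRandomUpgradableSpell filters the character's Gameplay Ability System abilities by the Abilities.Casting tag and a level below 2, then picks one at random.
; If one is found, the chest sets its level through the spec handle, prints the unlocked ability's class name and destroys itself.
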(event `self.ReceiveActorBeginOverlap`
  (params (OtherActor :type "Actor Object Reference"))
  (bind _asbp_element_character (cast `/Game/Characters/BP_ElementCharacter` OtherActor))
  (bind _elementabilitysystemcomponent (`ElementCharacterBase.ElementAbilitySystemComponent` _asbp_element_character))
  (bind (_returnvalue _foundupgrade) (`self.FindRandomUpgradableSpell` _elementabilitysystemcomponent))
  (if _foundupgrade
    (`ElementAbilitySystemComponent.SetAbilityLevelByHandle` _elementabilitysystemcomponent _returnvalue 2)
    (`KismetSystemLibrary.PrintString` (`KismetStringLibrary.Concat_StrStr` "Upgrade unlocked: " (`KismetSystemLibrary.GetClassDisplayName` (`GameplayStatics.GetObjectClass` (`.ReturnValue` (`AbilitySystemBlueprintLibrary.GetGameplayAbilityFromSpecHandle` _elementabilitysystemcomponent _returnvalue))))) true true (struct :`G` 0.66 :`B` 1.0 :`A` 1.0) 2.0 "Ability Upgrade")
    (`self.K2_DestroyActor`)))

(fn `FindRandomUpgradableSpell`
  (params (AbilitySystemComponent :type "ElementAbilitySystemComponent Object Reference"))
  (returns (ReturnValue :type "GameplayAbilitySpecHandle Structure") (FoundUpgrade :type Boolean))
  (locals (SpellAbilities :type "Array of GameplayAbilitySpecHandle Structure"))
  (bind (_outitem _outindex) (`KismetArrayLibrary.Array_Random` (`local.SpellAbilities`)))
  (bind _outabilityhandles (`AbilitySystemComponent.GetAllAbilities` AbilitySystemComponent))
  (for _array_element _outabilityhandles
    (if (and (`ElementAbilitySystemComponent.HasAssetTagByHandle` AbilitySystemComponent _array_element (struct :`TagName` "Abilities.Casting")) (< (`ElementAbilitySystemComponent.GetAbilityLevel` AbilitySystemComponent _array_element) 2))
      (`KismetArrayLibrary.Array_Add` (`local.SpellAbilities`) _array_element)))
  (return _outitem (> _outindex -1)))

(fn `UserConstructionScript`)