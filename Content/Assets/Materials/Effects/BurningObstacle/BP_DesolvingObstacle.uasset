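; Tree obstacle that dissolves and destroys itself once its assigned enemies have been killed.
; BeginPlay creates a dynamic dissolve material and binds to each assigned enemy's GAS health attribute change.
; Each change to zero health decrements EnemiesRemaining; at zero, a timeline animates the material's mask value before destroying the actor.
; GateZone overlap logic for gathering enemies and setting the count is disconnected, so neither is computed here.
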(event `OnHealthChanged`
  (params (AttributeSet :type "AttributeSet Object Reference") (OldValue :type "Float (single-precision)") (NewValue :type "Float (single-precision)"))
  (if (== NewValue 0.0)
    (`KismetSystemLibrary.PrintString` "Tree got OnEnemyKilled" true true (struct :`G` 0.66 :`B` 1.0 :`A` 1.0) 5.0)
    (bind _output_get (set `self.EnemiesRemaining` (- (`self.EnemiesRemaining`) 1)))
    (`KismetSystemLibrary.PrintString` (`KismetStringLibrary.Conv_IntToString` (`self.EnemiesRemaining`)) true true (struct :`G` 0.66 :`B` 1.0 :`A` 1.0) 5.0)
    (if (<= _output_get 0)
      (`self.StartDissolve`))))

(event `self.ReceiveBeginPlay`
  (bind _desolvingtree (`self.DesolvingTree`))
  (`PrimitiveComponent.SetMaterial` (`self.DesolvingTree`) 0 "/Game/Assets/Materials/Effects/BurningObstacle/DesolveMaterial/MI_ShamanStaff1_Desolve_Inst.MI_ShamanStaff1_Desolve_Inst")
  (bind _returnvalue (`PrimitiveComponent.CreateDynamicMaterialInstance` _desolvingtree 0 (`PrimitiveComponent.GetMaterial` _desolvingtree 0) "None"))
  (bind _output_get (set `self.treeMaterial` _returnvalue))
  (for _array_element (`self.AssignedEnemies`)
    (bind _returnvalue_2 (`AbilitySystemComponent.GetAttributeSet` (`ElementCharacterBase.ElementAbilitySystemComponent` _array_element) "/Script/Out_of_Your_Element.ElementHealthAttributeSet"))
    (add `ElementHealthAttributeSet.OnHealthChanged` _returnvalue_2 (delegate `OnHealthChanged`))))

(event `StartDissolve`
  (bind (_direction _desolvetrack) (`Timeline|Timeline`)
    (:`Update`
      (`MaterialInstanceDynamic.SetScalarParameterValue` (stale `self.ReceiveBeginPlay` _output_get) "MaskedValue" (`KismetMathLibrary.Lerp` 1.1 0.19 _desolvetrack)))
    (:`Finished`
      (`self.K2_DestroyActor`))))

(fn `UserConstructionScript`)