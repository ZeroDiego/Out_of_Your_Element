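; Tutorial event Blueprint that teaches attacking and element switching through a step counter and WBP_PopUp widgets.
; On BeginPlay it binds to the player BP_ElementCharacter's attack and element-changed delegates, which advance the steps while the tutorial is active.
; Each step shows a popup and clears older ones, with the last removed after a short delay.
; StartTutorial activates the sequence, but its only call here is unconnected.
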(event `OnAttackEvent`
  (params (AttackData :type "AttackData Structure"))
  (`KismetSystemLibrary.PrintString` "Attack")
  (if (and (`self.bTutorialActive`) (== (`self.TutorialStep`) 1))
    (set `self.TutorialStep` 2)
    (bind _returnvalue (`|CreateWidget` "/Game/UI/Popup/WBP_PopUp.WBP_PopUp_C" null "Great! You attacked. Now press Q or E to change your element."))
    (`UserWidget.AddToViewport` _returnvalue 0)
    (`self.RemoveOldWidgets` _returnvalue)))

(event `self.ReceiveBeginPlay`
  (bind _asbp_element_character (cast `/Game/Characters/BP_ElementCharacter` (`Controller.K2_GetPawn` (`GameplayStatics.GetPlayerController` 0))))
  (add `ElementCharacter.OnElementChangedDelegate` _asbp_element_character (delegate `OnElementChangedEvent`))
  (add `ElementCharacter.OnAttackDelegate` _asbp_element_character (delegate `OnAttackEvent`)))

(event `OnElementChangedEvent`
  (params (OldElement :type "Element Structure") (NewElement :type "Element Structure"))
  (`KismetSystemLibrary.PrintString` "Element Changed")
  (if (and (`self.bTutorialActive`) (== (`self.TutorialStep`) 2))
    (set `self.TutorialStep` 3)
    (bind _returnvalue (`|CreateWidget` "/Game/UI/Popup/WBP_PopUp.WBP_PopUp_C" null ""))
    (`UserWidget.AddToViewport` _returnvalue 0)
    (`self.RemoveOldWidgets` _returnvalue)
    (`KismetSystemLibrary.Delay` 2.0)
    (`Widget.RemoveFromParent` _returnvalue)))

(event `StartTutorial`
  (`KismetSystemLibrary.PrintString` "Tutorial")
  (set `self.bTutorialActive` true)
  (bind _returnvalue (`|CreateWidget` "/Game/UI/Popup/WBP_PopUp.WBP_PopUp_C" null ""))
  (`UserWidget.AddToViewport` _returnvalue 0)
  (set `self.TutorialStep` 1))

(fn `RemoveOldWidgets`
  (params (`New Widget` :type "Object Object Reference"))
  (bind _foundwidgets (`WidgetBlueprintLibrary.GetAllWidgetsOfClass` "/Game/UI/Popup/WBP_PopUp.WBP_PopUp_C"))
  (for _array_element _foundwidgets
    (if (not (== _array_element `New Widget`))
      (`Widget.RemoveFromParent` _array_element))))

(fn `UserConstructionScript`)