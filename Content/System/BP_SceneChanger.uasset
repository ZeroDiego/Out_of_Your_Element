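; BP_SceneChanger is a level-transition trigger that loads NextScene when a BP_ElementCharacter enters it.
; An optional check scans BP_AICharacterBase actors, blocking the change and creating a widget if any are alive.
; When CanChangeScene is true, it requests synchronous saves from the player controller, character and game instance before opening the level.
; BlocksMovement determines whether its collision component is enabled at BeginPlay.
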(event `self.ReceiveBeginPlay`
  (`PrimitiveComponent.SetCollisionEnabled` (`self.Collision`) (select `bool` (`self.bBlocksMovement`) :`false` "NoCollision" :`true` "QueryAndPhysics" :!type "ECollisionEnabled Enum"))
  (set `self.bOverlapActive` false))

(event `self.Trigger.OnComponentBeginOverlap`
  (params (OverlappedComponent :type "PrimitiveComponent Object Reference") (OtherActor :type "Actor Object Reference") (OtherComp :type "PrimitiveComponent Object Reference") (OtherBodyIndex :type Integer) (bFromSweep :type Boolean) (SweepResult :type "HitResult Structure (by ref)"))
  (bind _asbp_element_character (cast `/Game/Characters/BP_ElementCharacter` OtherActor))
  (bind _asbp_element_player_controller (cast `/Game/Characters/BP_ElementPlayerController` (`Pawn.GetLocalViewingPlayerController` _asbp_element_character)))
  (set `self.bFoundALivingEnemy` false)
  (if (`self.bCheckForEnemiesBeforeSceneChange`)
    (bind _outactors (`GameplayStatics.GetAllActorsOfClass` "/Game/AI/V1/BP_AICharacterBase.BP_AICharacterBase_C"))
    (for _array_element _outactors
      (if (not (`/Game/AI/V1/BP_AICharacterBase.bDead` _array_element))
        (set `self.bFoundALivingEnemy` true)))
    (if (`self.bFoundALivingEnemy`)
      (`self.CreateNewWidget`)
      (set `self.bCanChangeScene` false)
      (else
        (set `self.bCanChangeScene` true)
        (if (`self.bCanChangeScene`) :!label _label
          (message `/Game/Save/SaveGame/BPI_Persistence.RequestSave` _asbp_element_player_controller false false)
          (message `/Game/Save/SaveGame/BPI_Persistence.RequestSave` _asbp_element_character false false)
          (bind _asbp_element_game_instance (cast `/Game/System/BP_ElementGameInstance` (`GameplayStatics.GetGameInstance`)))
          (`/Game/System/BP_ElementGameInstance.RequestSave` _asbp_element_game_instance false false)
          (`GameplayStatics.OpenLevelBySoftObjectPtr` (`self.NextScene`)))))
    (else
      (goto _label))))

(fn `UserConstructionScript`)