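; Base Blueprint for a ranged AI enemy, animated with the Shaman Goblin anim Blueprint.
; The InRange pawn sensor writes a seen player character to the blackboard Target, replacing a deprecated AI Perception path, and StartAttack toggles the anim instance's IsAttacking flag.
; BeginPlay binds the GAS health attribute set's death event, which destroys the magic circle plane.
; The construction script pins the overlay widget to the mesh's Neck socket.
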(event `/Game/AI/BPI_EnemyActions.StartAttack`
  (bind _asabp_shaman_goblin (cast `/Game/Assets/Animations/Characters/Goblin/ShamanGoblin/ABP_Shaman_Goblin` (`SkeletalMeshComponent.GetAnimInstance` (`self.Mesh`))))
  (if (`/Game/Assets/Animations/Characters/Goblin/ShamanGoblin/ABP_Shaman_Goblin.bIsAttacking` _asabp_shaman_goblin)
    (set `/Game/Assets/Animations/Characters/Goblin/ShamanGoblin/ABP_Shaman_Goblin.bIsAttacking` false _asabp_shaman_goblin)
    (else
      (set `/Game/Assets/Animations/Characters/Goblin/ShamanGoblin/ABP_Shaman_Goblin.bIsAttacking` true _asabp_shaman_goblin))))

(event `self.InRange.OnSeePawn`
  (params (Pawn :type "Pawn Object Reference"))
  ; Kollar om spelaren är inrange för projectile attacker
  (bind _asbp_element_character (cast `/Game/Characters/BP_ElementCharacter` Pawn))
  (`BlackboardComponent.SetValueAsObject` (`AIBlueprintHelperLibrary.GetBlackboard` (`AIBlueprintHelperLibrary.GetAIController` self)) "Target" _asbp_element_character))

(event `self.ReceiveBeginPlay`
  (`parent.ReceiveBeginPlay`)
  (bind _returnvalue (`AbilitySystemComponent.GetAttributeSet` (`self.ElementAbilitySystemComponent`) "/Script/Out_of_Your_Element.ElementHealthAttributeSet"))
  (add `ElementHealthAttributeSet.OnDeath` _returnvalue (delegate `OnDeathEvent`)))

(event `OnDeathEvent`
  (params (DyingActor :type "Actor Object Reference") (DamageTaken :type "DamageTaken Structure (by ref)"))
  (`ActorComponent.K2_DestroyComponent` (`self.MagicCirclePLane`)))

(event `self.AIPerception_Chase.OnTargetPerceptionUpdated`
  (params (Actor :type "Actor Object Reference") (Stimulus :type "AIStimulus Structure"))
  ; Deprecated
)

(fn `UserConstructionScript`
  (`SceneComponent.K2_AttachToComponent` (`self.OverlayWidget`) (`self.Mesh`) "Neck" "KeepRelative" "SnapToTarget" "SnapToTarget" true))