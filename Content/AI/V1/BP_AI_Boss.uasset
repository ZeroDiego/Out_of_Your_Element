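; Boss AI character that runs a three-phase elemental fight (Nature, Water, Fire) on the Gameplay Ability System.
; Stage events, plus a totem phase resisting all three elements, swap tracked SetByCaller effects granting elemental resistance or healing.
; Health-change bindings fire once per threshold, notifying BP_BossManager and changing the hit montage and magic circle material.
; The final threshold sets the death animation flag, then shows the end credits and unpossesses the player.
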(event `Stage1`
  (for _array_element (`self.Active Handles`)
    (`AbilitySystemComponent.RemoveActiveGameplayEffect` (`self.ElementAbilitySystemComponent`) _array_element -1))
  (bind _returnvalue (`AbilitySystemBlueprintLibrary.MakeSpecHandleByClass` "/Game/GameplayEffects/Attribute/GE_NatureAttribute_SetByCaller.GE_NatureAttribute_SetByCaller_C"))
  (bind _returnvalue_2 (`AbilitySystemBlueprintLibrary.AssignTagSetByCallerMagnitude` _returnvalue (struct :`TagName` "Abilities.Parameters.Resistance.Percent") 1.0))
  (bind _returnvalue_3 (`AbilitySystemComponent.BP_ApplyGameplayEffectSpecToSelf` (`self.ElementAbilitySystemComponent`) _returnvalue_2))
  (`KismetArrayLibrary.Array_Add` (`self.Active Handles`) _returnvalue_3)
  (bind _returnvalue_4 (`AbilitySystemBlueprintLibrary.MakeSpecHandleByClass` "/Game/GameplayEffects/Attribute/GE_WaterAttribute_SetByCaller.GE_WaterAttribute_SetByCaller_C"))
  (bind _returnvalue_5 (`AbilitySystemBlueprintLibrary.AssignTagSetByCallerMagnitude` _returnvalue_4 (struct :`TagName` "Abilities.Parameters.Heal.Percent") 2.0))
  (bind _returnvalue_6 (`AbilitySystemComponent.BP_ApplyGameplayEffectSpecToSelf` (`self.ElementAbilitySystemComponent`) _returnvalue_5))
  (`KismetArrayLibrary.Array_Add` (`self.Active Handles`) _returnvalue_6))

(event `self.ReceiveBeginPlay`
  (`parent.ReceiveBeginPlay`)
  (bind _returnvalue (`AbilitySystemComponent.GetAttributeSet` (`self.ElementAbilitySystemComponent`) "/Script/Out_of_Your_Element.ElementHealthAttributeSet"))
  (add `ElementHealthAttributeSet.OnHealthChanged` _returnvalue (delegate `Stage 1 Defeated`))
  (add `ElementHealthAttributeSet.OnHealthChanged` _returnvalue (delegate `Stage 2 Defeated`))
  (add `ElementHealthAttributeSet.OnHealthChanged` _returnvalue (delegate `Stage 3 Defeated`))
  (`PrimitiveComponent.SetMaterial` (`self.MagicCirclePLane`) 0 "/Game/Assets/Materials/Effects/MagicCircles/M_Nature_Magic_Circle.M_Nature_Magic_Circle"))

(event `Stage 1 Defeated`
  (params (AttributeSet :type "AttributeSet Object Reference") (OldValue :type "Float (single-precision)") (NewValue :type "Float (single-precision)"))
  (if (<= NewValue (`self.Stage 1 Health`))
    (`/Engine/EditorBlueprintResources/StandardMacros.DoOnce` false
      (:`Completed`
        (bind _returnvalue (`GameplayStatics.GetActorOfClass` "/Game/AI/V1/BP_BossManager.BP_BossManager_C"))
        (`/Game/AI/V1/BP_BossManager.NatureDefeated` _returnvalue)
        (`self.PlayAnimMontage` "/Game/Assets/Animations/Characters/Boss/AM_Boss_Take_Damage.AM_Boss_Take_Damage")
        (`PrimitiveComponent.SetMaterial` (`self.MagicCirclePLane`) 0 "/Game/Assets/Materials/Effects/MagicCircles/M_Water_Magic_Circle.M_Water_Magic_Circle")))))

(event `Stage2`
  (for _array_element (`self.Active Handles`)
    (`AbilitySystemComponent.RemoveActiveGameplayEffect` (`self.ElementAbilitySystemComponent`) _array_element -1))
  (bind _returnvalue (`AbilitySystemBlueprintLibrary.MakeSpecHandleByClass` "/Game/GameplayEffects/Attribute/GE_WaterAttribute_SetByCaller.GE_WaterAttribute_SetByCaller_C"))
  (bind _returnvalue_2 (`AbilitySystemBlueprintLibrary.AssignTagSetByCallerMagnitude` _returnvalue (struct :`TagName` "Abilities.Parameters.Resistance.Percent") 1.0))
  (bind _returnvalue_3 (`AbilitySystemComponent.BP_ApplyGameplayEffectSpecToSelf` (`self.ElementAbilitySystemComponent`) _returnvalue_2))
  (`KismetArrayLibrary.Array_Add` (`self.Active Handles`) _returnvalue_3)
  (bind _returnvalue_4 (`AbilitySystemBlueprintLibrary.MakeSpecHandleByClass` "/Game/GameplayEffects/Attribute/GE_FireAttribute_SetByCaller.GE_FireAttribute_SetByCaller_C"))
  (bind _returnvalue_5 (`AbilitySystemBlueprintLibrary.AssignTagSetByCallerMagnitude` _returnvalue_4 (struct :`TagName` "Abilities.Parameters.Resistance.Percent") 1.0))
  (bind _returnvalue_6 (`AbilitySystemComponent.BP_ApplyGameplayEffectSpecToSelf` (`self.ElementAbilitySystemComponent`) _returnvalue_5))
  (`KismetArrayLibrary.Array_Add` (`self.Active Handles`) _returnvalue_6))

(event `Stage 2 Defeated`
  (params (AttributeSet :type "AttributeSet Object Reference") (OldValue :type "Float (single-precision)") (NewValue :type "Float (single-precision)"))
  (if (<= NewValue (`self.Stage 2 Health`))
    (`/Engine/EditorBlueprintResources/StandardMacros.DoOnce` false
      (:`Completed`
        (bind _returnvalue (`GameplayStatics.GetActorOfClass` "/Game/AI/V1/BP_BossManager.BP_BossManager_C"))
        (`/Game/AI/V1/BP_BossManager.WaterDefeated` _returnvalue)
        (`self.PlayAnimMontage` "/Game/Assets/Animations/Characters/Boss/AM_Boss_Take_Damage.AM_Boss_Take_Damage")
        (`PrimitiveComponent.SetMaterial` (`self.MagicCirclePLane`) 0 "/Game/Assets/Materials/Effects/MagicCircles/M_Fire_Magic_Circle.M_Fire_Magic_Circle")))))

(event `Stage3`
  (for _array_element (`self.Active Handles`)
    (`AbilitySystemComponent.RemoveActiveGameplayEffect` (`self.ElementAbilitySystemComponent`) _array_element -1))
  (bind _returnvalue (`AbilitySystemBlueprintLibrary.MakeSpecHandleByClass` "/Game/GameplayEffects/Attribute/GE_FireAttribute_SetByCaller.GE_FireAttribute_SetByCaller_C"))
  (bind _returnvalue_2 (`AbilitySystemBlueprintLibrary.AssignTagSetByCallerMagnitude` _returnvalue (struct :`TagName` "Abilities.Parameters.Resistance.Percent") 1.0))
  (bind _returnvalue_3 (`AbilitySystemComponent.BP_ApplyGameplayEffectSpecToSelf` (`self.ElementAbilitySystemComponent`) _returnvalue_2))
  (`KismetArrayLibrary.Array_Add` (`self.Active Handles`) _returnvalue_3)
  (bind _returnvalue_4 (`AbilitySystemBlueprintLibrary.MakeSpecHandleByClass` "/Game/GameplayEffects/Attribute/GE_NatureAttribute_SetByCaller.GE_NatureAttribute_SetByCaller_C"))
  (bind _returnvalue_5 (`AbilitySystemBlueprintLibrary.AssignTagSetByCallerMagnitude` _returnvalue_4 (struct :`TagName` "Abilities.Parameters.Heal.Percent") 2.0))
  (bind _returnvalue_6 (`AbilitySystemComponent.BP_ApplyGameplayEffectSpecToSelf` (`self.ElementAbilitySystemComponent`) _returnvalue_5))
  (`KismetArrayLibrary.Array_Add` (`self.Active Handles`) _returnvalue_6))

(event `Stage 3 Defeated`
  (params (AttributeSet :type "AttributeSet Object Reference") (OldValue :type "Float (single-precision)") (NewValue :type "Float (single-precision)"))
  (bind _returnvalue (`GameplayStatics.GetPlayerController` 0))
  (if (<= NewValue (`self.Stage 3 Health`))
    (`/Engine/EditorBlueprintResources/StandardMacros.DoOnce` false
      (:`Completed`
        (bind _returnvalue_2 (`GameplayStatics.GetActorOfClass` "/Game/AI/V1/BP_BossManager.BP_BossManager_C"))
        (`/Game/AI/V1/BP_BossManager.FireDefeated` _returnvalue_2)
        (bind _asabp_boss (cast `/Game/Assets/Animations/Characters/Boss/ABP_Boss` (`SkeletalMeshComponent.GetAnimInstance` (`self.Mesh`))))
        (set `/Game/Assets/Animations/Characters/Boss/ABP_Boss.bIsDead` true _asabp_boss)
        (`KismetSystemLibrary.Delay` 8.0)
        (bind _returnvalue_3 (`|CreateWidget` "/Game/UI/Menus/EndCredits/WBP_EndCredits.WBP_EndCredits_C"))
        (`UserWidget.AddToViewport` _returnvalue_3 0)
        (`WidgetBlueprintLibrary.SetInputMode_UIOnlyEx` _returnvalue _returnvalue_3)
        (`Controller.UnPossess` _returnvalue)))))

(event `TotemStages`
  (for _array_element (`self.Active Handles`)
    (`AbilitySystemComponent.RemoveActiveGameplayEffect` (`self.ElementAbilitySystemComponent`) _array_element -1))
  (bind _returnvalue (`AbilitySystemBlueprintLibrary.MakeSpecHandleByClass` "/Game/GameplayEffects/Attribute/GE_NatureAttribute_SetByCaller.GE_NatureAttribute_SetByCaller_C"))
  (bind _returnvalue_2 (`AbilitySystemBlueprintLibrary.AssignTagSetByCallerMagnitude` _returnvalue (struct :`TagName` "Abilities.Parameters.Resistance.Percent") 1.0))
  (bind _returnvalue_3 (`AbilitySystemComponent.BP_ApplyGameplayEffectSpecToSelf` (`self.ElementAbilitySystemComponent`) _returnvalue_2))
  (`KismetArrayLibrary.Array_Add` (`self.Active Handles`) _returnvalue_3)
  (bind _returnvalue_4 (`AbilitySystemBlueprintLibrary.MakeSpecHandleByClass` "/Game/GameplayEffects/Attribute/GE_WaterAttribute_SetByCaller.GE_WaterAttribute_SetByCaller_C"))
  (bind _returnvalue_5 (`AbilitySystemBlueprintLibrary.AssignTagSetByCallerMagnitude` _returnvalue_4 (struct :`TagName` "Abilities.Parameters.Resistance.Percent") 1.0))
  (bind _returnvalue_6 (`AbilitySystemComponent.BP_ApplyGameplayEffectSpecToSelf` (`self.ElementAbilitySystemComponent`) _returnvalue_5))
  (`KismetArrayLibrary.Array_Add` (`self.Active Handles`) _returnvalue_6)
  (bind _returnvalue_7 (`AbilitySystemBlueprintLibrary.MakeSpecHandleByClass` "/Game/GameplayEffects/Attribute/GE_FireAttribute_SetByCaller.GE_FireAttribute_SetByCaller_C"))
  (bind _returnvalue_8 (`AbilitySystemBlueprintLibrary.AssignTagSetByCallerMagnitude` _returnvalue_7 (struct :`TagName` "Abilities.Parameters.Resistance.Percent") 1.0))
  (bind _returnvalue_9 (`AbilitySystemComponent.BP_ApplyGameplayEffectSpecToSelf` (`self.ElementAbilitySystemComponent`) _returnvalue_8))
  (`KismetArrayLibrary.Array_Add` (`self.Active Handles`) _returnvalue_9))

(fn `UserConstructionScript`
  (`parent.UserConstructionScript`))