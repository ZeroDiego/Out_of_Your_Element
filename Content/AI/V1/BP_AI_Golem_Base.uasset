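; BP_AI_Golem_Base is a golem AI base Blueprint that targets element characters and drives attack animation state.
; Actor overlap with a BP_ElementCharacter writes it to the AI controller's Blackboard "Target" key, and ending the overlap clears that key.
; StartAttack toggles IsAttacking on the ABP_Golem anim instance rather than only setting it.
; An overlay widget attaches to the mesh's Neck socket at construction and again, fully snapped, on BeginPlay.
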(event `self.ReceiveBeginPlay`
  (`parent.ReceiveBeginPlay`)
  (`SceneComponent.K2_AttachToComponent` (`self.OverlayWidget`) (`self.Mesh`) "Neck" "SnapToTarget" "SnapToTarget" "SnapToTarget" true))

(event `self.ReceiveActorBeginOverlap`
  (params (OtherActor :type "Actor Object Reference"))
  (bind _returnvalue (`AIBlueprintHelperLibrary.GetBlackboard` (`AIBlueprintHelperLibrary.GetAIController` self)))
  (bind _asbp_element_character (cast `/Game/Characters/BP_ElementCharacter` OtherActor))
  (`/Engine/EditorBlueprintResources/StandardMacros.IsValid` _returnvalue
    (:`Is Valid`
      (`BlackboardComponent.SetValueAsObject` _returnvalue "Target" _asbp_element_character))))

(event `self.ReceiveActorEndOverlap`
  (params (OtherActor :type "Actor Object Reference"))
  (bind _returnvalue (`AIBlueprintHelperLibrary.GetBlackboard` (`AIBlueprintHelperLibrary.GetAIController` self)))
  (cast `/Game/Characters/BP_ElementCharacter` OtherActor)
  (`/Engine/EditorBlueprintResources/StandardMacros.IsValid` _returnvalue
    (:`Is Valid`
      (`BlackboardComponent.SetValueAsObject` _returnvalue "Target" null))))

(event `self.StartAttack`
  (bind _asabp_golem (cast `/Game/Assets/Animations/Characters/Golem/ABP_Golem` (`SkeletalMeshComponent.GetAnimInstance` (`self.Mesh`))))
  (if (`/Game/Assets/Animations/Characters/Golem/ABP_Golem.bIsAttacking` _asabp_golem)
    (set `/Game/Assets/Animations/Characters/Golem/ABP_Golem.bIsAttacking` false _asabp_golem)
    (else
      (set `/Game/Assets/Animations/Characters/Golem/ABP_Golem.bIsAttacking` true _asabp_golem))))

(fn `UserConstructionScript`
  (`SceneComponent.K2_AttachToComponent` (`self.OverlayWidget`) (`self.Mesh`) "Neck" "KeepRelative" "SnapToTarget" "SnapToTarget" true))