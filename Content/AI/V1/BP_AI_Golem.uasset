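; Golem AI enemy that targets element characters entering its overlap range and drives its attack animation.
; Overlap events set the blackboard Target to the BP_ElementCharacter and clear it when one leaves.
; StartAttack toggles IsAttacking on ABP_Golem rather than only setting it.
; An overlay widget attaches to the mesh's Neck socket in construction and again on BeginPlay, which also prints the class name.
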(event `self.ReceiveBeginPlay`
  (`KismetSystemLibrary.PrintString` (`KismetSystemLibrary.GetClassDisplayName` (`GameplayStatics.GetObjectClass` self)))
  (`parent.ReceiveBeginPlay`)
  (`SceneComponent.K2_AttachToComponent` (`self.OverlayWidget`) (`self.Mesh`) "Neck" "SnapToTarget" "SnapToTarget" "SnapToTarget" true))

(event `self.ReceiveActorBeginOverlap`
  (params (OtherActor :type "Actor Object Reference"))
  (bind _asbp_element_character (cast `/Game/Characters/BP_ElementCharacter` OtherActor))
  (`BlackboardComponent.SetValueAsObject` (`AIBlueprintHelperLibrary.GetBlackboard` (`AIBlueprintHelperLibrary.GetAIController` self)) "Target" _asbp_element_character))

(event `self.ReceiveActorEndOverlap`
  (params (OtherActor :type "Actor Object Reference"))
  (cast `/Game/Characters/BP_ElementCharacter` OtherActor)
  (`BlackboardComponent.SetValueAsObject` (`AIBlueprintHelperLibrary.GetBlackboard` (`AIBlueprintHelperLibrary.GetAIController` self)) "Target" null))

(event `self.StartAttack`
  (bind _asabp_golem (cast `/Game/Assets/Animations/Characters/Golem/ABP_Golem` (`SkeletalMeshComponent.GetAnimInstance` (`self.Mesh`))))
  (if (`/Game/Assets/Animations/Characters/Golem/ABP_Golem.bIsAttacking` _asabp_golem)
    (set `/Game/Assets/Animations/Characters/Golem/ABP_Golem.bIsAttacking` false _asabp_golem)
    (else
      (set `/Game/Assets/Animations/Characters/Golem/ABP_Golem.bIsAttacking` true _asabp_golem))))

(fn `UserConstructionScript`
  (`SceneComponent.K2_AttachToComponent` (`self.OverlayWidget`) (`self.Mesh`) "Neck" "KeepRelative" "SnapToTarget" "SnapToTarget" true))