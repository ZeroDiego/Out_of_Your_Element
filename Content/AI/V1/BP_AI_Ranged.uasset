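; Ranged enemy AI Blueprint that feeds sightings of BP_ElementCharacter into its AI controller's Blackboard.
; PawnSensing sets CanSeePlayerCharacter and TargetLocation, while AIPerception sets or clears Target as sensing succeeds or fails.
; A second sensor, InRange, also writes Target but reuses the perception handler's cast result instead of its own pawn.
; Health changes arrive through the ability system's HealthAttributeSet, and zero health only prints a death message.
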(event `self.ReceiveBeginPlay`
  (bind _returnvalue (`AbilitySystemComponent.GetAttributeSet` (`self.ElementAbilitySystemComponent`) "/Script/Out_of_Your_Element.HealthAttributeSet"))
  (add `HealthAttributeSet.OnHealthChanged` _returnvalue (delegate `OnHealthChanged`)))

(event `OnHealthChanged`
  (params (AttributeSet :type "AttributeSet Object Reference") (OldValue :type "Float (single-precision)") (NewValue :type "Float (single-precision)"))
  (if (== NewValue 0.0)
    (`KismetSystemLibrary.PrintString` "Enemy died!")))

(event `self.PawnSensing.OnSeePawn`
  (params (Pawn :type "Pawn Object Reference"))
  (bind _returnvalue (`AIBlueprintHelperLibrary.GetBlackboard` (`AIBlueprintHelperLibrary.GetAIController` self)))
  (bind _asbp_element_character (cast `/Game/Characters/BP_ElementCharacter` Pawn))
  (`BlackboardComponent.SetValueAsBool` _returnvalue "CanSeePlayerCharacter" true)
  (`BlackboardComponent.SetValueAsVector` _returnvalue "TargetLocation" (`self.K2_GetActorLocation` _asbp_element_character)))

(event `self.AIPerception.OnPerceptionUpdated`
  (params (UpdatedActors :type "Array of Actor Object Reference (by ref)")))

(event `self.InRange.OnSeePawn`
  (params (Pawn :type "Pawn Object Reference"))
  (cast `/Game/Characters/BP_ElementCharacter` Pawn)
  (`BlackboardComponent.SetValueAsObject` (`AIBlueprintHelperLibrary.GetBlackboard` (`AIBlueprintHelperLibrary.GetAIController` self)) "Target" (stale `self.AIPerception.OnTargetPerceptionUpdated` _asbp_element_character) :!label _label))

(event `self.AIPerception.OnTargetPerceptionUpdated`
  (params (Actor :type "Actor Object Reference") (Stimulus :type "AIStimulus Structure"))
  (bind _asbp_element_character (cast `/Game/Characters/BP_ElementCharacter` Actor))
  (if (`.bSuccessfullySensed` (break `AIStimulus` Stimulus))
    (goto _label)
    (else
      (`BlackboardComponent.SetValueAsObject` (`AIBlueprintHelperLibrary.GetBlackboard` (`AIBlueprintHelperLibrary.GetAIController` self)) "Target" null))))

(fn `UserConstructionScript`)