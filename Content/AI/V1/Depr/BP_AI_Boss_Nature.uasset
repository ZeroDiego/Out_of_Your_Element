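; Nature boss AI Blueprint that reports its defeat to BP_BossManager.
; On BeginPlay it binds to the element health attribute set and, when health reaches zero, calls NatureDefeated once.
; A key-press event clears tracked Gameplay Effects, applies SetByCaller water and fire resistance effects, stores their handles and prints a debug message.
; An unconnected chain would apply nature resistance and a water-attribute heal effect, but never runs.
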(event `Press`
  (for _array_element (`self.Active Handles`)
    (`AbilitySystemComponent.RemoveActiveGameplayEffect` (`self.ElementAbilitySystemComponent`) _array_element -1))
  (bind _returnvalue (`AbilitySystemBlueprintLibrary.MakeSpecHandleByClass` "/Game/GameplayEffects/Attribute/GE_WaterAttribute_SetByCaller.GE_WaterAttribute_SetByCaller_C"))
  (bind _returnvalue_2 (`AbilitySystemBlueprintLibrary.AssignTagSetByCallerMagnitude` _returnvalue (struct :`TagName` "Abilities.Parameters.Resistance.Percent") 1.0))
  (bind _returnvalue_3 (`AbilitySystemComponent.BP_ApplyGameplayEffectSpecToSelf` (`self.ElementAbilitySystemComponent`) _returnvalue_2))
  (`KismetArrayLibrary.Array_Add` (`self.Active Handles`) _returnvalue_3)
  (bind _returnvalue_4 (`AbilitySystemBlueprintLibrary.MakeSpecHandleByClass` "/Game/GameplayEffects/Attribute/GE_FireAttribute_SetByCaller.GE_FireAttribute_SetByCaller_C"))
  (bind _returnvalue_5 (`AbilitySystemBlueprintLibrary.AssignTagSetByCallerMagnitude` _returnvalue_4 (struct :`TagName` "Abilities.Parameters.Resistance.Percent") 1.0))
  (bind _returnvalue_6 (`AbilitySystemComponent.BP_ApplyGameplayEffectSpecToSelf` (`self.ElementAbilitySystemComponent`) _returnvalue_5))
  (`KismetArrayLibrary.Array_Add` (`self.Active Handles`) _returnvalue_6)
  (`KismetSystemLibrary.PrintText` "ö pressed"))

(event `self.ReceiveBeginPlay`
  (`parent.ReceiveBeginPlay`)
  (bind _returnvalue (`AbilitySystemComponent.GetAttributeSet` (`self.ElementAbilitySystemComponent`) "/Script/Out_of_Your_Element.ElementHealthAttributeSet"))
  (add `ElementHealthAttributeSet.OnHealthChanged` _returnvalue (delegate `BossStageDeath`)))

(event `BossStageDeath`
  (params (AttributeSet :type "AttributeSet Object Reference") (OldValue :type "Float (single-precision)") (NewValue :type "Float (single-precision)"))
  (if (== NewValue 0.0)
    (`/Engine/EditorBlueprintResources/StandardMacros.DoOnce` false
      (:`Completed`
        (bind _returnvalue (`GameplayStatics.GetActorOfClass` "/Game/AI/V1/BP_BossManager.BP_BossManager_C"))
        (`/Game/AI/V1/BP_BossManager.NatureDefeated` _returnvalue)))))

(fn `UserConstructionScript`
  (`parent.UserConstructionScript`))