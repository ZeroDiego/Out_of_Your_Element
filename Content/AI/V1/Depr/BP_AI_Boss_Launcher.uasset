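; Boss launcher AI that swaps its single elemental attack by phase: rock throw, water gun or fireball.
; Each phase event clears the ability system component and grants that phase's ability, with keys Ö, Å and Ä triggering them manually.
; BeginPlay writes a point ahead of the actor to the LauncherTarget blackboard key.
; Tick checks the totem manager's phase but takes no action, and older ability-assignment logic is left disconnected.
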(event `SetPhase1Stats`
  (bind _elementabilitysystemcomponent (`self.ElementAbilitySystemComponent`))
  (`AbilitySystemComponent.ClearAllAbilities` _elementabilitysystemcomponent)
  (`AbilitySystemComponent.K2_GiveAbility` _elementabilitysystemcomponent "/Game/GameplayAbilities/Spell/Base/GA_RockThrow.GA_RockThrow_C" 0 -1))

(event `self.ReceiveBeginPlay`
  (bind _output_get (set `self.Firing Direction` (+ (`self.K2_GetActorLocation`) (* (`self.GetActorForwardVector`) (`self.NewVar`)))))
  (`BlackboardComponent.SetValueAsVector` (`AIBlueprintHelperLibrary.GetBlackboard` (`AIBlueprintHelperLibrary.GetAIController` self)) "LauncherTarget" _output_get))

(event `SetPhase2Stats`
  (bind _elementabilitysystemcomponent (`self.ElementAbilitySystemComponent`))
  (`AbilitySystemComponent.ClearAllAbilities` _elementabilitysystemcomponent)
  (`AbilitySystemComponent.K2_GiveAbility` _elementabilitysystemcomponent "/Game/GameplayAbilities/Spell/Base/GA_WaterGun.GA_WaterGun_C" 0 -1))

(event `Key|ö`
  (params (Key :type "Key Structure"))
  (:`Pressed`
    (`self.SetPhase1Stats`)))

(event `Key|å`
  (params (Key :type "Key Structure"))
  (:`Pressed`
    (`self.SetPhase2Stats`)))

(event `SetPhase3Stats`
  (bind _elementabilitysystemcomponent (`self.ElementAbilitySystemComponent`))
  (`AbilitySystemComponent.ClearAllAbilities` _elementabilitysystemcomponent)
  (`AbilitySystemComponent.K2_GiveAbility` _elementabilitysystemcomponent "/Game/GameplayAbilities/Spell/Base/GA_Fireball.GA_Fireball_C" 0 -1))

(event `Key|ä`
  (params (Key :type "Key Structure"))
  (:`Pressed`
    (`self.SetPhase3Stats`)))

(event `self.ReceiveTick`
  (params (DeltaSeconds :type "Float (single-precision)"))
  (bind _returnvalue (`GameplayStatics.GetActorOfClass` "/Game/AI/V1/BP_TotemManager.BP_TotemManager_C"))
  (bind _currentphase (`/Game/AI/V1/BP_TotemManager.CurrentPhase` _returnvalue))
  (if (== _currentphase 0)
    _
    (elif (== _currentphase 1)
      _
      (elif (== _currentphase 2)
        _))))

(fn `UserConstructionScript`
  (`parent.UserConstructionScript`))