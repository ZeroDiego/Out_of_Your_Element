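; Boss manager actor that runs a staged Nature, Water and Fire boss fight, spawning each boss at its own location.
; Water and Fire spawns are guarded to happen once.
; Nature and Water defeats spawn next-element totems at four TotemSpawn markers and reconfigure the projectile spawner's projectile, directions and fire interval.
; Fire's defeat prints victory and clears the projectile class, looked up through ProjectileSpawner rather than the BP_ProjectileSpawner used elsewhere.
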(event `SpawnBoss`
  (`|SpawnActorFromClass` :`Class` "/Game/AI/V1/BP_AI_Boss_Nature.BP_AI_Boss_Nature_C" :`SpawnTransform` (`KismetMathLibrary.Conv_VectorToTransform` (`self.K2_GetActorLocation`)) :`CollisionHandlingOverride` "Undefined" :`TransformScaleMethod` "MultiplyWithRoot" :`Instigator` null)
  (`KismetSystemLibrary.PrintString` "BossSpawned")
  (bind _returnvalue (`GameplayStatics.GetActorOfClass` "/Game/AI/BP_ProjectileSpawner.BP_ProjectileSpawner_C"))
  (set `ProjectileSpawner.bEnableLeft` true _returnvalue)
  (set `ProjectileSpawner.bEnableRight` true _returnvalue))

(event `self.ReceiveBeginPlay`)

(event `SpawnWater`
  (if (not (`self.WaterSpawned`))
    (`|SpawnActorFromClass` :`Class` "/Game/AI/V1/BP_AI_Boss_Water.BP_AI_Boss_Water_C" :`SpawnTransform` (`KismetMathLibrary.Conv_VectorToTransform` (`self.K2_GetActorLocation`)) :`CollisionHandlingOverride` "Undefined" :`TransformScaleMethod` "MultiplyWithRoot" :`Instigator` null)
    (set `self.WaterSpawned` true)))

(event `SpawnFire`
  (if (not (`self.FireSpawned`))
    (`|SpawnActorFromClass` :`Class` "/Game/AI/V1/BP_AI_Boss_Fire.BP_AI_Boss_Fire_C" :`SpawnTransform` (`KismetMathLibrary.Conv_VectorToTransform` (`self.K2_GetActorLocation`)) :`CollisionHandlingOverride` "Undefined" :`TransformScaleMethod` "MultiplyWithRoot" :`Instigator` null)
    (set `self.FireSpawned` true)))

(event `NatureDefeated`
  (set `self.Nature Defeated` true)
  (`KismetSystemLibrary.PrintString` "Nature Defeated")
  (bind _returnvalue (`GameplayStatics.GetActorOfClass` "/Game/AI/V1/TotemSpawn1.TotemSpawn1_C"))
  (`|SpawnActorFromClass` :`Class` "/Game/AI/V1/BP_BossTotem_Water.BP_BossTotem_Water_C" :`SpawnTransform` (`KismetMathLibrary.Conv_VectorToTransform` (`self.K2_GetActorLocation` _returnvalue)) :`CollisionHandlingOverride` "Undefined" :`TransformScaleMethod` "MultiplyWithRoot" :`Instigator` null)
  (`KismetSystemLibrary.PrintString` "Totem spawned")
  (bind _returnvalue_2 (`GameplayStatics.GetActorOfClass` "/Game/AI/V1/TotemSpawn2.TotemSpawn2_C"))
  (`|SpawnActorFromClass` :`Class` "/Game/AI/V1/BP_BossTotem_Water.BP_BossTotem_Water_C" :`SpawnTransform` (`KismetMathLibrary.Conv_VectorToTransform` (`self.K2_GetActorLocation` _returnvalue_2)) :`CollisionHandlingOverride` "Undefined" :`TransformScaleMethod` "MultiplyWithRoot" :`Instigator` null)
  (`KismetSystemLibrary.PrintString` "Totem spawned")
  (bind _returnvalue_3 (`GameplayStatics.GetActorOfClass` "/Game/AI/V1/TotemSpawn3.TotemSpawn3_C"))
  (`|SpawnActorFromClass` :`Class` "/Game/AI/V1/BP_BossTotem_Water.BP_BossTotem_Water_C" :`SpawnTransform` (`KismetMathLibrary.Conv_VectorToTransform` (`self.K2_GetActorLocation` _returnvalue_3)) :`CollisionHandlingOverride` "Undefined" :`TransformScaleMethod` "MultiplyWithRoot" :`Instigator` null)
  (`KismetSystemLibrary.PrintString` "Totem spawned")
  (bind _returnvalue_4 (`GameplayStatics.GetActorOfClass` "/Game/AI/V1/TotemSpawn4.TotemSpawn4_C"))
  (`|SpawnActorFromClass` :`Class` "/Game/AI/V1/BP_BossTotem_Water.BP_BossTotem_Water_C" :`SpawnTransform` (`KismetMathLibrary.Conv_VectorToTransform` (`self.K2_GetActorLocation` _returnvalue_4)) :`CollisionHandlingOverride` "Undefined" :`TransformScaleMethod` "MultiplyWithRoot" :`Instigator` null)
  (`KismetSystemLibrary.PrintString` "Totem spawned")
  (bind _returnvalue_5 (`GameplayStatics.GetActorOfClass` "/Game/AI/BP_ProjectileSpawner.BP_ProjectileSpawner_C"))
  (set `ProjectileSpawner.ProjectileClass` "/Game/Projectiles/BP_WaterGunProjectile.BP_WaterGunProjectile_C" _returnvalue_5)
  (set `ProjectileSpawner.bEnableLeft` false _returnvalue_5)
  (set `ProjectileSpawner.bEnableRight` false _returnvalue_5)
  (set `ProjectileSpawner.bEnableUp` true _returnvalue_5)
  (set `ProjectileSpawner.bEnableDown` true _returnvalue_5)
  (set `ProjectileSpawner.FireInterval` (`/Game/AI/BP_ProjectileSpawner.FireIntervalBeforeTotems` _returnvalue_5) _returnvalue_5))

(event `WaterDefeated`
  (set `self.Water Defeated` true)
  (`KismetSystemLibrary.PrintString` "Water Defeated")
  (bind _returnvalue (`GameplayStatics.GetActorOfClass` "/Game/AI/V1/TotemSpawn1.TotemSpawn1_C"))
  (`|SpawnActorFromClass` :`Class` "/Game/AI/V1/BP_BossTotem_Fire.BP_BossTotem_Fire_C" :`SpawnTransform` (`KismetMathLibrary.Conv_VectorToTransform` (`self.K2_GetActorLocation` _returnvalue)) :`CollisionHandlingOverride` "Undefined" :`TransformScaleMethod` "MultiplyWithRoot" :`Instigator` null)
  (`KismetSystemLibrary.PrintString` "Totem spawned")
  (bind _returnvalue_2 (`GameplayStatics.GetActorOfClass` "/Game/AI/V1/TotemSpawn2.TotemSpawn2_C"))
  (`|SpawnActorFromClass` :`Class` "/Game/AI/V1/BP_BossTotem_Fire.BP_BossTotem_Fire_C" :`SpawnTransform` (`KismetMathLibrary.Conv_VectorToTransform` (`self.K2_GetActorLocation` _returnvalue_2)) :`CollisionHandlingOverride` "Undefined" :`TransformScaleMethod` "MultiplyWithRoot" :`Instigator` null)
  (`KismetSystemLibrary.PrintString` "Totem spawned")
  (bind _returnvalue_3 (`GameplayStatics.GetActorOfClass` "/Game/AI/V1/TotemSpawn3.TotemSpawn3_C"))
  (`|SpawnActorFromClass` :`Class` "/Game/AI/V1/BP_BossTotem_Fire.BP_BossTotem_Fire_C" :`SpawnTransform` (`KismetMathLibrary.Conv_VectorToTransform` (`self.K2_GetActorLocation` _returnvalue_3)) :`CollisionHandlingOverride` "Undefined" :`TransformScaleMethod` "MultiplyWithRoot" :`Instigator` null)
  (`KismetSystemLibrary.PrintString` "Totem spawned")
  (bind _returnvalue_4 (`GameplayStatics.GetActorOfClass` "/Game/AI/V1/TotemSpawn4.TotemSpawn4_C"))
  (`|SpawnActorFromClass` :`Class` "/Game/AI/V1/BP_BossTotem_Fire.BP_BossTotem_Fire_C" :`SpawnTransform` (`KismetMathLibrary.Conv_VectorToTransform` (`self.K2_GetActorLocation` _returnvalue_4)) :`CollisionHandlingOverride` "Undefined" :`TransformScaleMethod` "MultiplyWithRoot" :`Instigator` null)
  (`KismetSystemLibrary.PrintString` "Totem spawned")
  (bind _returnvalue_5 (`GameplayStatics.GetActorOfClass` "/Game/AI/BP_ProjectileSpawner.BP_ProjectileSpawner_C"))
  (set `ProjectileSpawner.ProjectileClass` "/Game/Projectiles/BP_FireballProjectile.BP_FireballProjectile_C" _returnvalue_5)
  (set `ProjectileSpawner.bEnableLeft` true _returnvalue_5)
  (set `ProjectileSpawner.bEnableRight` true _returnvalue_5)
  (set `ProjectileSpawner.bEnableUp` true _returnvalue_5)
  (set `ProjectileSpawner.bEnableDown` true _returnvalue_5)
  (set `ProjectileSpawner.FireInterval` (`/Game/AI/BP_ProjectileSpawner.FireIntervalBeforeTotems` _returnvalue_5) _returnvalue_5))

(event `FireDefeated`
  (set `self.Fire Defeated` true)
  (`KismetSystemLibrary.PrintString` "Victory")
  (bind _returnvalue (`GameplayStatics.GetActorOfClass` "/Script/Out_of_Your_Element.ProjectileSpawner"))
  (set `ProjectileSpawner.ProjectileClass` null _returnvalue))

(fn `UserConstructionScript`)