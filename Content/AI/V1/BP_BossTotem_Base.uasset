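; BP_BossTotem_Base is a base Blueprint for boss totems, giving them an overhead health overlay and death on zero health.
; On BeginPlay it binds to the health attribute set from its ability system component, creates the enemy overlay widget from that set, and applies GoblinMaxWalkSpeed to character movement.
; When health reaches zero, a DoOnce guard triggers a short delay before destroying the actor.
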(event `self.ReceiveBeginPlay`
  (bind _returnvalue (`AbilitySystemComponent.GetAttributeSet` (`self.ElementAbilitySystemComponent`) "/Script/Out_of_Your_Element.ElementHealthAttributeSet"))
  (add `ElementHealthAttributeSet.OnHealthChanged` _returnvalue (delegate `OnHealthChanged`))
  (bind _returnvalue_2 (`|CreateWidget` "/Game/UI/World/WBP_EnemyOverlay.WBP_EnemyOverlay_C" null _returnvalue))
  (`WidgetComponent.SetWidget` (`self.OverlayWidget`) _returnvalue_2)
  (set `CharacterMovementComponent.MaxWalkSpeed` (`self.Goblin_MaxWalkSpeed`) (`self.CharacterMovement`)))

(event `OnHealthChanged`
  (params (AttributeSet :type "AttributeSet Object Reference") (OldValue :type "Float (single-precision)") (NewValue :type "Float (single-precision)"))
  (if (== NewValue 0.0)
    (`/Engine/EditorBlueprintResources/StandardMacros.DoOnce` false
      (:`Completed`
        (`KismetSystemLibrary.Delay` 0.1)
        (`self.K2_DestroyActor`)))))

(fn `UserConstructionScript`)