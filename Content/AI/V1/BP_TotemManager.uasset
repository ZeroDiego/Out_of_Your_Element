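; BP_TotemManager tracks destroyed Nature, Water and Fire totems and triggers boss spawns.
; Each totem event increments its own counter and, from four onward, calls SpawnBoss, SpawnWater or SpawnFire on BP_BossManager.
; Nature and Water also advance CurrentPhase, while Fire only prints it.
; Debug prints report counts and phase, and disconnected nodes hold unused phase-stat updates for BP_AI_Boss_Launcher.
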(event `self.ReceiveBeginPlay`)

(event `OnNatureTotemDestroyed`
  (bind _output_get (set `self.Destroyed Nature Totem` (+ (`self.Destroyed Nature Totem`) 1)))
  (`KismetSystemLibrary.PrintString` (`KismetStringLibrary.Conv_IntToString` _output_get))
  (if (>= (`self.Destroyed Nature Totem`) 4)
    (bind _output_get_2 (set `self.CurrentPhase` (+ (`self.CurrentPhase`) 1)))
    (`KismetSystemLibrary.PrintString` (`KismetStringLibrary.Conv_IntToString` _output_get_2))
    (`KismetSystemLibrary.PrintString` "Phase:")
    (bind _returnvalue (`GameplayStatics.GetActorOfClass` "/Game/AI/V1/BP_BossManager.BP_BossManager_C"))
    (`/Game/AI/V1/BP_BossManager.SpawnBoss` _returnvalue)))

(event `OnWaterTotemDestroyed`
  (bind _output_get (set `self.Destroyed Water Totem` (+ (`self.Destroyed Water Totem`) 1)))
  (`KismetSystemLibrary.PrintString` (`KismetStringLibrary.Conv_IntToString` _output_get))
  (if (>= (`self.Destroyed Water Totem`) 4)
    (bind _output_get_2 (set `self.CurrentPhase` (+ (`self.CurrentPhase`) 1)))
    (`KismetSystemLibrary.PrintString` (`KismetStringLibrary.Conv_IntToString` _output_get_2))
    (`KismetSystemLibrary.PrintString` "Phase:")
    (bind _returnvalue (`GameplayStatics.GetActorOfClass` "/Game/AI/V1/BP_BossManager.BP_BossManager_C"))
    (`/Game/AI/V1/BP_BossManager.SpawnWater` _returnvalue)))

(event `OnFireTotemDestroyed`
  (bind _output_get (set `self.Destroyed Fire Totems` (+ (`self.Destroyed Fire Totems`) 1)))
  (`KismetSystemLibrary.PrintString` (`KismetStringLibrary.Conv_IntToString` _output_get))
  (if (>= (`self.Destroyed Fire Totems`) 4)
    (`KismetSystemLibrary.PrintString` (`KismetStringLibrary.Conv_IntToString` (`self.CurrentPhase`)))
    (`KismetSystemLibrary.PrintString` "Phase:")
    (bind _returnvalue (`GameplayStatics.GetActorOfClass` "/Game/AI/V1/BP_BossManager.BP_BossManager_C"))
    (`/Game/AI/V1/BP_BossManager.SpawnFire` _returnvalue)))

(fn `UserConstructionScript`)