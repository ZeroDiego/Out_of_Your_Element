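; Water boss AI Blueprint that reports its defeat to the boss manager.
; On BeginPlay it runs the parent logic and binds BossStageDeath to the health-changed event of the ElementHealthAttributeSet on its ability system component.
; When health reaches zero, a DoOnce gate lets it find BP_BossManager in the level and call WaterDefeated a single time.
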(event `self.ReceiveBeginPlay`
  (`parent.ReceiveBeginPlay`)
  (bind _returnvalue (`AbilitySystemComponent.GetAttributeSet` (`self.ElementAbilitySystemComponent`) "/Script/Out_of_Your_Element.ElementHealthAttributeSet"))
  (add `ElementHealthAttributeSet.OnHealthChanged` _returnvalue (delegate `BossStageDeath`)))

(event `BossStageDeath`
  (params (AttributeSet :type "AttributeSet Object Reference") (OldValue :type "Float (single-precision)") (NewValue :type "Float (single-precision)"))
  (if (== NewValue 0.0)
    (`/Engine/EditorBlueprintResources/StandardMacros.DoOnce` false
      (:`Completed`
        (bind _returnvalue (`GameplayStatics.GetActorOfClass` "/Game/AI/V1/BP_BossManager.BP_BossManager_C"))
        (`/Game/AI/V1/BP_BossManager.WaterDefeated` _returnvalue)))))

(fn `UserConstructionScript`
  (`parent.UserConstructionScript`))