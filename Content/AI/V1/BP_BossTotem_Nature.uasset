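; BP_BossTotem_Nature is the nature boss totem, which reports its own destruction to the totem manager.
; On BeginPlay it binds to health changes on its ability system's ElementHealthAttributeSet.
; When health reaches zero, a DoOnce finds BP_TotemManager in the level and calls OnNatureTotemDestroyed, with debug prints for the lookup and a failed cast.
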(event `self.ReceiveBeginPlay`
  (`parent.ReceiveBeginPlay`)
  (bind _returnvalue (`AbilitySystemComponent.GetAttributeSet` (`self.ElementAbilitySystemComponent`) "/Script/Out_of_Your_Element.ElementHealthAttributeSet"))
  (add `ElementHealthAttributeSet.OnHealthChanged` _returnvalue (delegate `CustomEvent_1`)))

(event `CustomEvent_1`
  (params (AttributeSet :type "AttributeSet Object Reference") (OldValue :type "Float (single-precision)") (NewValue :type "Float (single-precision)"))
  (if (== NewValue 0.0)
    (`/Engine/EditorBlueprintResources/StandardMacros.DoOnce` false
      (:`Completed`
        (bind _returnvalue (`GameplayStatics.GetActorOfClass` "/Game/AI/V1/BP_TotemManager.BP_TotemManager_C"))
        (`KismetSystemLibrary.PrintString` "Manager Found")
        (bind _asbp_totem_manager (cast `/Game/AI/V1/BP_TotemManager` _returnvalue)
          (:`then`
            (`/Game/AI/V1/BP_TotemManager.OnNatureTotemDestroyed` _asbp_totem_manager))
          (:`CastFailed`
            (`KismetSystemLibrary.PrintString` "Cast failed")))))))

(fn `UserConstructionScript`
  (`parent.UserConstructionScript`))