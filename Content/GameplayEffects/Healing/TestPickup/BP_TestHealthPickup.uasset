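; BP_TestHealthPickup is a test health pickup that applies the GE_HealthPickup gameplay effect to a BP_ElementCharacter entering its trigger.
; On overlap it plays a pickup sound, applies the effect through the character's Ability System Component, then destroys itself.
; On BeginPlay it creates a dynamic material on its sphere, and a timeline drives aura strength and opacity to create a pulse.
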(event `self.PickupTrigger.OnComponentBeginOverlap`
  (params (OverlappedComponent :type "PrimitiveComponent Object Reference") (OtherActor :type "Actor Object Reference") (OtherComp :type "PrimitiveComponent Object Reference") (OtherBodyIndex :type Integer) (bFromSweep :type Boolean) (SweepResult :type "HitResult Structure (by ref)"))
  (bind _asbp_element_character (cast `/Game/Characters/BP_ElementCharacter` OtherActor))
  (`GameplayStatics.PlaySoundAtLocation` "/Game/Assets/Audio/SoundWaves/Pickups/A_Pickup.A_Pickup" (`self.K2_GetActorLocation`) (struct) 1.0 1.0 0.0 null null null null)
  (`AbilitySystemComponent.BP_ApplyGameplayEffectToSelf` :`self` (`AbilitySystemBlueprintLibrary.GetAbilitySystemComponent` _asbp_element_character) :`GameplayEffectClass` "/Game/GameplayEffects/Healing/GE_HealthPickup.GE_HealthPickup_C")
  (`self.K2_DestroyActor`))

(event `self.ReceiveBeginPlay`
  (bind _returnvalue (`PrimitiveComponent.CreateDynamicMaterialInstance` (`self.Sphere`) 0 null "None"))
  (set `self.auraMID` _returnvalue)
  (bind (_direction _pulse) (`Timeline|TL_AuraPulse`)
    (:`Update`
      (`MaterialInstanceDynamic.SetScalarParameterValue` (`self.auraMID`) "AuraStrength" (`KismetMathLibrary.Lerp` 1.5 5.0 _pulse))
      (`MaterialInstanceDynamic.SetScalarParameterValue` (`self.auraMID`) "Opacity" (`KismetMathLibrary.Lerp` 0.06 0.14 _pulse)))))

(fn `UserConstructionScript`)